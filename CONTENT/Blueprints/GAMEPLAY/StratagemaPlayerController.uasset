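; Stratagema player controller that sets up a local player's match and manages its chat, score and game-over UI.
; On BeginPlay it loads level and player saves, sets GameMode spawn points, spawns grid nodes and requests the pawn spawn.
; Chat relays through the GameMode's controller list to each controller's widget, with T/Tab toggling chat and cursor.
; GameOver pauses, shows its widget, then quits under SteamDebug or returns to lobby.
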(event `Create Grid`
  ;[1 1 1] Create Grid
  (for _array_element (`.MyLevelGridLocations_27_DA685ABF4EC53D5ACBE02B9A33955A4E` (break `/Game/Blueprints/AllLevels/StratagemaLevelInfo` (`self.LevelSettings`)))
    (`|SpawnActorFromClass` "/Game/Blueprints/Pawns/StratagemaGridNode.StratagemaGridNode_C" (`KismetMathLibrary.Conv_VectorToTransform` _array_element) "AlwaysSpawn" "OverrideRootScale")))

(event `self.ReceiveBeginPlay`
  ;[1 1 1] Loads Player & Level Information
  (if (`self.IsLocalController`)
    (`WidgetLayoutLibrary.RemoveAllWidgets`)
    (`self.LoadGame`)
    (`self.PassPlayerInfoToServer` (`self.PlayerSettings`))
    (`self.Create Grid`)))

(event `PassPlayerInfoToServer`
  (params (PlayerInformation :type "/Game/Blueprints/AllLevels/StratagemaPlayerInfo Structure"))
  ;[1 1 1] Passes Information to Spawn
  (set `self.PlayerSettings` PlayerInformation)
  (bind _asstratageme_game_mode (cast `/Game/Blueprints/GamePlay/StratagemeGameMode` (`GameplayStatics.GetGameMode`)))
  (`/Game/Blueprints/GamePlay/StratagemeGameMode.SpawnPlayer` _asstratageme_game_mode self (`.MyPlayerPawn_11_DA685ABF4EC53D5ACBE02B9A33955A4E` (break `/Game/Blueprints/AllLevels/StratagemaPlayerInfo` (`self.PlayerSettings`))))
  (`self.SetupChatWindow`)
  (`self.Setup Score HUD`))

(event `self.ReceiveTick`
  (params (DeltaSeconds :type "Float (single-precision)"))
  (bind _asstratageme_game_mode (cast `/Game/Blueprints/GamePlay/StratagemeGameMode` (`GameplayStatics.GetGameMode`))))

(event `SetAllPlayersSpawned`
  ;[1 1 1] Have All Players Been Spawned (ON by Default)
  (set `self.HaveAllPlayersSpawned` true))

(event `Setup Score HUD`
  ;[1 1 1] Show Score HUD
  (bind _returnvalue (`|CreateWidget` "/Game/Widgets/GamePlay/Player1ScoreWB.Player1ScoreWB_C"))
  (`Widget.SetVisibility` _returnvalue "Visible" :!label _label)
  (set `self.GamePlayScoreWB` _returnvalue :!label _label_2)
  (`UserWidget.AddToViewport` _returnvalue 0))

(event `SetupChatWindow`
  ;[1 1 1] Show Gameplay Chat
  (bind _returnvalue (`|CreateWidget` "/Game/Widgets/AllLevels/GameplayChat.GameplayChat_C"))
  (`Widget.SetVisibility` _returnvalue "Hidden")
  (bind _output_get (set `self.GamePlayChatWB` _returnvalue))
  (`UserWidget.AddToViewport` _output_get 0))

(event `Key|Z`
  (params (Key :type "Key Structure" :default "AnyKey"))
  ;[1 1 1] Show Score HUD
  (:`Pressed`
    (`KismetSystemLibrary.PrintString` "Hello")
    (`/Engine/EditorBlueprintResources/StandardMacros.FlipFlop`
      (:`A`
        (`Widget.SetVisibility` (stale `Setup Score HUD` _returnvalue) "Hidden")
        (goto _label_2))
      (:`B`
        (goto _label)))))

(event `GetChatMessage`
  (params (TextToSend :type Text))
  ;[1 1 1] Process Chat
  (set `self.SenderText` TextToSend)
  (set `self.SenderName` (`.MyPlayerName_8_0AAD31484FF23DBC49F602A131948E20` (break `/Game/Blueprints/AllLevels/StratagemaPlayerInfo` (`self.PlayerSettings`))))
  (bind _asstratageme_game_mode (cast `/Game/Blueprints/GamePlay/StratagemeGameMode` (`GameplayStatics.GetGameMode`)))
  (for _array_element (`/Game/Blueprints/GamePlay/StratagemeGameMode.AllPlayerControls` _asstratageme_game_mode)
    (bind _asstratagema_player_controller (cast `/Game/Blueprints/GAMEPLAY/StratagemaPlayerController` _array_element))
    (`self.UpdateChat` _asstratagema_player_controller (`self.SenderName`) (`self.SenderText`))))

(event `UpdateChat`
  (params (SenderName :type Text) (SenderText :type Text))
  ;[1 1 1] Update Chat on Client
  (`/Game/Widgets/AllLevels/ChatWindow.UpdateChatWindow` (`/Game/Widgets/AllLevels/GameplayChat.GameplayChat` (`self.GamePlayChatWB`)) SenderName SenderText))

(event `Key|T`
  (params (Key :type "Key Structure" :default "AnyKey"))
  (bind _gameplaychatwb (`self.GamePlayChatWB`))
  ;[1 1 1] 'T' for Menu / Mouse
  (:`Pressed`
    (`/Engine/EditorBlueprintResources/StandardMacros.FlipFlop` :!label _label_3
      (:`A`
        (set `self.bShowMouseCursor` true)
        (`Widget.SetVisibility` _gameplaychatwb "Visible"))
      (:`B`
        (set `self.bShowMouseCursor` false)
        (`Widget.SetVisibility` _gameplaychatwb "Hidden")))))

(event `GameOver`
  ;[1 1 1] Game Over
  (`GameplayStatics.SetGamePaused` true)
  (`Widget.RemoveFromParent` (`self.GamePlayScoreWB`))
  (bind _returnvalue (`|CreateWidget` "/Game/Widgets/GamePlay/GameOverWB.GameOverWB_C"))
  (`UserWidget.AddToViewport` _returnvalue 0)
  (`KismetSystemLibrary.Delay` 5.0)
  (bind _asstratageme_game_mode (cast `/Game/Blueprints/GamePlay/StratagemeGameMode` (`GameplayStatics.GetGameMode`)))
  (if (`/Game/Blueprints/GamePlay/StratagemeGameMode.SteamDebug` _asstratageme_game_mode)
    (`KismetSystemLibrary.ExecuteConsoleCommand` "Quit")
    (else
      (`/Game/Blueprints/GamePlay/StratagemeGameMode.ReturnToLobby` _asstratageme_game_mode))))

(event `Key|Tab`
  (params (Key :type "Key Structure" :default "AnyKey"))
  ;[1 1 1] 'T' for Menu / Mouse
  (:`Pressed`
    (goto _label_3)))

(fn `LoadGame`
  (`|ExecutionSequence`
    (:`then_0`
      (bind _returnvalue (`GameplayStatics.LoadGameFromSlot` (`self.LevelSettingsSave`)))
      (bind _asstratagema_level_save_game (cast `/Game/Blueprints/AllLevels/StratagemaLevelSaveGame` _returnvalue))
      (bind _s_levelinfo (`/Game/Blueprints/AllLevels/StratagemaLevelSaveGame.S_LevelInfo` _asstratagema_level_save_game))
      (set `self.LevelSettings` _s_levelinfo)
      (bind _asstratageme_game_mode (cast `/Game/Blueprints/GamePlay/StratagemeGameMode` (`GameplayStatics.GetGameMode`)))
      (bind (_mylevelname _mylevelgridlocations _player1startposition _player2startposition _player3startposition) (break `/Game/Blueprints/AllLevels/StratagemaLevelInfo` _s_levelinfo))
      (set `/Game/Blueprints/GamePlay/StratagemeGameMode.Player1SpawnPoint` (`KismetMathLibrary.MakeTransform` (.location _player1startposition) (struct :`Yaw` 45.0) (1.2 1.2 1.2)) _asstratageme_game_mode)
      (set `/Game/Blueprints/GamePlay/StratagemeGameMode.Player2SpawnPoint` (`KismetMathLibrary.MakeTransform` (.location _player2startposition) (struct :`Roll` 180.0) (1.2 1.2 1.2)) _asstratageme_game_mode)
      (set `/Game/Blueprints/GamePlay/StratagemeGameMode.Player3SpawnPoint` (`KismetMathLibrary.MakeTransform` (.location _player3startposition) (struct :`Yaw` 180.0) (1.2 1.2 1.2)) _asstratageme_game_mode))
    (:`then_1`
      (bind _returnvalue_2 (`GameplayStatics.LoadGameFromSlot` (`self.PlayerSettingsSave`)))
      (bind _asstratagema_save_game (cast `/Game/Blueprints/AllLevels/StratagemaSaveGame` _returnvalue_2))
      (set `self.PlayerSettings` (`/Game/Blueprints/AllLevels/StratagemaSaveGame.S_PlayerInfo` _asstratagema_save_game)))))

(fn `UserConstructionScript`)