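; Game mode for a timed match of up to three players, holding their scores.
; SpawnPlayer matches controllers by actor order, then spawns and possesses pawns at per-player points, using fixed classes under SteamDebug.
; Tick counts down the level-settings length and calls the first controller's GameOver at zero.
; Its own GameOver pauses, shows the end widget, then server-travels to Lobby or quits under SteamDebug; logout triggers session destruction.
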(event `self.ReceiveBeginPlay`
  ;[1 1 1] Set Game Lenght in Seconds
  (bind _asstratagema_player_controller (cast `/Game/Blueprints/GamePlay/StratagemaPlayerController` (`GameplayStatics.GetPlayerController` 0)))
  (bind (_levelsettings_mylevelname _levelsettings_mylevelgridlocations _levelsettings_player1startposition _levelsettings_player2startposition _levelsettings_player3startposition _levelsettings_gamelenght) (break `/Game/Blueprints/AllLevels/StratagemaLevelInfo` (`/Game/Blueprints/GamePlay/StratagemaPlayerController.LevelSettings` _asstratagema_player_controller)))
  (bind _output_get (set `self.GameLenght` (`KismetStringLibrary.Conv_StringToDouble` (`KismetTextLibrary.Conv_TextToString` _levelsettings_gamelenght)))))

(event `SpawnPlayer`
  (params (PlayerController :type "PlayerController Object Reference") (PlayerPawn :type "Pawn Class Reference"))
  (bind _steamdebug (`self.SteamDebug`))
  (bind _playerarray (`GameState.PlayerArray` (`GameplayStatics.GetGameState`)))
  ;[1 1 1] Set Player Controllers & ID
  (bind _outactors (`GameplayStatics.GetAllActorsOfClass` "/Script/Engine.PlayerController"))
  (set `self.Player1Contoller` (`KismetArrayLibrary.Array_Get` _outactors))
  (set `self.Player1ID` (`PlayerState.PlayerId` (`KismetArrayLibrary.Array_Get` _playerarray)))
  (set `self.Player2Contoller` (`KismetArrayLibrary.Array_Get` _outactors 1))
  (set `self.Player2ID` (`PlayerState.PlayerId` (`KismetArrayLibrary.Array_Get` _playerarray 1)))
  (set `self.Player3Contoller` (`KismetArrayLibrary.Array_Get` _outactors 2))
  (set `self.Player3ID` (`PlayerState.PlayerId` (`KismetArrayLibrary.Array_Get` _playerarray 2)))
  ;[1 1 1] Set Player Start Position
  (if (== PlayerController (`self.Player1Contoller`))
    (set `self.StartPosition` (`self.Player1SpawnPoint`))
    (if _steamdebug
      ;[1 1 0] Player 1
      (bind _returnvalue (`|SpawnActorFromClass` "/Game/Blueprints/Pawns/Player1.Player1_C" (`self.Player1SpawnPoint`) "AlwaysSpawn" "OverrideRootScale"))
      (`/Engine/EditorBlueprintResources/StandardMacros.IsValid` _returnvalue :!label _label
        (:`Is Valid`
          (`Controller.Possess` (`self.Player1Contoller`) _returnvalue))
        (:`Is Not Valid`
          (`KismetSystemLibrary.Delay` 0.2)
          (goto _label)))
      (else
        ;[1 0.5 0.5] Spawn Player Original
        (bind _returnvalue_2 (`|SpawnActorFromClass` PlayerPawn (`self.StartPosition`) "AlwaysSpawn" "OverrideRootScale" :!label _label_2))
        (`Controller.Possess` PlayerController _returnvalue_2)))
    (elif (== PlayerController (`self.Player2Contoller`))
      (set `self.StartPosition` (`self.Player2SpawnPoint`))
      (if _steamdebug
        ;[0 1 1] Player 2
        (bind _returnvalue_3 (`|SpawnActorFromClass` "/Game/Blueprints/Pawns/Player2.Player2_C" (`self.Player2SpawnPoint`) "AlwaysSpawn" "OverrideRootScale"))
        (`/Engine/EditorBlueprintResources/StandardMacros.IsValid` _returnvalue_3 :!label _label_3
          (:`Is Valid`
            (`Controller.Possess` (`self.Player2Contoller`) _returnvalue_3))
          (:`Is Not Valid`
            (`KismetSystemLibrary.Delay` 0.2)
            (goto _label_3)))
        (else
          (goto _label_2)))
      (elif (== PlayerController (`self.Player3Contoller`))
        (set `self.StartPosition` (`self.Player3SpawnPoint`))
        (if _steamdebug
          ;[1 0 1] Player 3
          (bind _returnvalue_4 (`|SpawnActorFromClass` "/Game/Blueprints/Pawns/Player3.Player3_C" (`self.Player3SpawnPoint`) "AlwaysSpawn" "OverrideRootScale"))
          (`/Engine/EditorBlueprintResources/StandardMacros.IsValid` _returnvalue_4 :!label _label_4
            (:`Is Valid`
              (`Controller.Possess` (`self.Player3Contoller`) _returnvalue_4))
            (:`Is Not Valid`
              (`KismetSystemLibrary.Delay` 0.2)
              (goto _label_4)))
          (else
            (goto _label_2)))))))

(event `self.ReceiveTick`
  (params (DeltaSeconds :type "Float (single-precision)"))
  ;[1 1 1] Timer
  (set `self.GameLenght` (- (`self.GameLenght`) DeltaSeconds))
  (if (<= (`self.GameLenght`) 0.0)
    (set `self.GameLenght` 0.0)
    (bind _asstratagema_player_controller (cast `/Game/Blueprints/GamePlay/StratagemaPlayerController` (`GameplayStatics.GetPlayerController` 0)))
    (`/Game/Blueprints/GamePlay/StratagemaPlayerController.GameOver` _asstratagema_player_controller)))

(event `self.K2_OnLogout`
  (params (ExitingController :type "Controller Object Reference"))
  ;[1 1 1] Event on Logout
  (bind _asstratagema_player_controller (cast `/Game/Blueprints/GamePlay/StratagemaPlayerController` ExitingController))
  (`/Game/Blueprints/AllLevels/StratagemaGameInstance.DestroySessionCaller` (cast `/Game/Blueprints/AllLevels/StratagemaGameInstance` (`GameplayStatics.GetGameInstance`) :!pure true) _asstratagema_player_controller))

(event `Update Player 1 Score`
  (params (Score :type Integer))
  ;[1 1 1] Player Scores Update System
  (bind _output_get (set `self.Player1Score` Score)))

(event `Update Player 2 Score`
  (params (Score :type Integer))
  ;[1 1 1] Player Scores Update System
  (bind _output_get (set `self.Player2Score` Score)))

(event `GameOver`
  ;[1 1 1] Game Over
  (`GameplayStatics.SetGamePaused` true)
  (bind _asstratagema_player_controller (cast `/Game/Blueprints/GamePlay/StratagemaPlayerController` (`GameplayStatics.GetPlayerController` 0))
    (:`then`
      (`Widget.RemoveFromParent` (`/Game/Blueprints/GamePlay/StratagemaPlayerController.GamePlayScoreWB` _asstratagema_player_controller))
      (bind _returnvalue (`|CreateWidget` "/Game/Widgets/GamePlay/GameOverWB.GameOverWB_C"))
      (`UserWidget.AddToViewport` _returnvalue 0)
      (`KismetSystemLibrary.Delay` 5.0)
      (if (`self.SteamDebug`)
        (`KismetSystemLibrary.ExecuteConsoleCommand` "Quit")
        (else
          (`self.ReturnToLobby`))))
    (:`CastFailed`
      (`KismetSystemLibrary.PrintString` "Cast Failed"))))

(event `ReturnToLobby`
  ;[1 1 1] On Game Over
  (`KismetSystemLibrary.ExecuteConsoleCommand` "servertravel /Game/Maps/Lobby" (`GameplayStatics.GetPlayerController` 0)))

(event `UpdatePlayer3Score`
  (params (Score :type Integer))
  ;[1 1 1] Player Scores Update System
  (bind _output_get (set `self.Player3Score` Score)))

(fn `UserConstructionScript`)