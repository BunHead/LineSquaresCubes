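; Lobby game mode for Stratagema that manages joining players, pawn selection, map settings, kicking and server travel to the game map.
; PostLogin registers controllers and initializes their lobby menus from game instance and map settings.
; UpdateEveryone pushes the player list, counts and available pawns to every controller and sets ReadyToStart from pawn choices, while logout frees the leaver's pawn.
; SwapPawn respawns and possesses pawns at three spawn points chosen by controller order.
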(event `SwapPawn`
  (params (PlayerController :type "PlayerController Object Reference") (PawnClass :type "Pawn Class Reference") (ChangedStatus :type Boolean))
  (bind _returnvalue (`Controller.K2_GetPawn` PlayerController))
  (bind _playerarray (`GameState.PlayerArray` (`GameplayStatics.GetGameState`)))
  ;[1 0.605 0.605] Swaps Pawn
  (bind _outactors (`GameplayStatics.GetAllActorsOfClass` "/Script/Engine.PlayerController"))
  (set `self.Player1Contoller` (`KismetArrayLibrary.Array_Get` _outactors))
  (set `self.Player2Contoller` (`KismetArrayLibrary.Array_Get` _outactors 1))
  (set `self.Player3Contoller` (`KismetArrayLibrary.Array_Get` _outactors 2))
  (for _array_element _playerarray
    (set `self.Player1ID` (`PlayerState.PlayerId` (`KismetArrayLibrary.Array_Get` _playerarray)))
    (set `self.Player2ID` (`PlayerState.PlayerId` (`KismetArrayLibrary.Array_Get` _playerarray 1)))
    (set `self.Player3ID` (`PlayerState.PlayerId` (`KismetArrayLibrary.Array_Get` _playerarray 2))))
  (if (not ChangedStatus)
    (`/Engine/EditorBlueprintResources/StandardMacros.IsValid` _returnvalue
      (:`Is Valid`
        (`self.K2_DestroyActor` _returnvalue))
      (:`Is Not Valid`
        _))
    (if (== PlayerController (`self.Player1Contoller`))
      ;[0 1 1] Server
      (bind _returnvalue_2 (`|SpawnActorFromClass` PawnClass (`self.Player1SpawnPoint`) "AlwaysSpawn" "OverrideRootScale"))
      (`Controller.Possess` PlayerController _returnvalue_2)
      (elif (== PlayerController (`self.Player2Contoller`))
        ;[0 1 1] Client 1
        (bind _returnvalue_3 (`|SpawnActorFromClass` PawnClass (`self.Player2SpawnPoint`) "AlwaysSpawn" "OverrideRootScale"))
        (`Controller.Possess` PlayerController _returnvalue_3)
        (else
          ;[0 1 1] Client 2
          (bind _returnvalue_4 (`|SpawnActorFromClass` PawnClass (`self.Player3SpawnPoint`) "AlwaysSpawn" "OverrideRootScale"))
          (`Controller.Possess` PlayerController _returnvalue_4))))))

(event `RespawnPlayer`
  (params (PlayerController :type "PlayerController Object Reference"))
  ;[1 0.46 0.46] Spawn Player
)

(event `self.K2_PostLogin`
  (params (NewPlayer :type "PlayerController Object Reference"))
  ;[0.495 1 0.495] Initial Setup
  ;;[1 1 1] Add Score Here = Auth = server
  (`/Engine/EditorBlueprintResources/ActorMacros.Switch Has Authority`
    (:`Authority`
      (`KismetArrayLibrary.Array_Add` (`self.AllPlayerController`) NewPlayer)
      (bind _outactors (`GameplayStatics.GetAllActorsOfClass` "/Script/Engine.PlayerStart"))
      (set `self.SpawnPoints` _outactors)
      (bind _asstratagema_game_instance (cast `/Game/Blueprints/AllLevels/StratagemaGameInstance` (`GameplayStatics.GetGameInstance`)))
      (set `self.ServerName` (`/Game/Blueprints/AllLevels/StratagemaGameInstance.SeverName` _asstratagema_game_instance))
      (set `self.MaxPlayers` (`/Game/Blueprints/AllLevels/StratagemaGameInstance.MaxPlayers` _asstratagema_game_instance))
      (bind _aslobby_player_controller (cast `/Game/Blueprints/Lobby/LobbyPlayerController` NewPlayer))
      (`/Game/Blueprints/Lobby/LobbyPlayerController.InitialSetup` _aslobby_player_controller)
      (`/Game/Blueprints/Lobby/LobbyPlayerController.SetupLobbyMenu` _aslobby_player_controller (`self.ServerName`))
      (`/Game/Blueprints/Lobby/LobbyPlayerController.UpdateLobbySettings` _aslobby_player_controller (`self.GameModeImage`) (`self.GameModeMapName`) (`self.GameModeMapTime`)))))

(event `AddToKickedList`
  ;[1 1 1] Add to Kick List
  (bind _aslobby_player_controller (cast `/Game/Blueprints/Lobby/LobbyPlayerController` (`GameplayStatics.GetPlayerController` 0)))
  (bind _lobbymenuwb (`/Game/Blueprints/Lobby/LobbyPlayerController.LobbyMenuWB` _aslobby_player_controller))
  (`/Engine/EditorBlueprintResources/StandardMacros.IsValid` _lobbymenuwb
    (:`Is Valid`
      (bind _gamesettings (`/Game/Widgets/Lobby/LobbyMenu.GameSettings` _lobbymenuwb))
      (if (`Widget.IsVisible` _gamesettings)
        (`/Game/Widgets/Lobby/GameSettings.FillPlayerWindow` _gamesettings)))))

(event `self.K2_OnLogout`
  (params (ExitingController :type "Controller Object Reference"))
  (bind _allplayercontroller (`self.AllPlayerController`))
  ;[1 1 1] On Logout Removes From Arrays
  (for (_array_element _array_index) _allplayercontroller
    (if (== _array_element ExitingController)
      (break)))
  (bind _aslobby_player_controller (cast `/Game/Blueprints/Lobby/LobbyPlayerController` (`KismetArrayLibrary.Array_Get` _allplayercontroller _array_index)))
  (`KismetArrayLibrary.Array_Set` (`self.AvailablePawns`) (`/Game/Blueprints/Lobby/LobbyPlayerController.SelectedPawn` _aslobby_player_controller) false)
  (`KismetArrayLibrary.Array_Remove` (`self.AllPlayerController`) _array_index)
  (`KismetArrayLibrary.Array_Remove` (`self.ConnectedPlayers`) _array_index)
  (`self.UpdateEveryone`))

(event `UpdateEveryone`
  (bind _allplayercontroller (`self.AllPlayerController`))
  ;[1 1 1] Updates Connected Players
  (bind _output_get (set `self.CurrentPlayers` (`KismetArrayLibrary.Array_Length` (`self.AllPlayerController`))))
  (if (> _output_get 0)
    (`KismetArrayLibrary.Array_Clear` (`self.ConnectedPlayers`))
    (for _array_element _allplayercontroller
      (bind _aslobby_player_controller (cast `/Game/Blueprints/Lobby/LobbyPlayerController` _array_element))
      (`KismetArrayLibrary.Array_Add` (`self.ConnectedPlayers`) (`/Game/Blueprints/Lobby/LobbyPlayerController.PlayerSettings` _aslobby_player_controller))
      (`/Game/Blueprints/Lobby/LobbyPlayerController.UpdateNumberOfPlayers` _aslobby_player_controller (`self.CurrentPlayers`) (`self.MaxPlayers`)))
    (for _array_element_2 _allplayercontroller
      (bind _aslobby_player_controller_2 (cast `/Game/Blueprints/Lobby/LobbyPlayerController` _array_element_2))
      (`/Game/Blueprints/Lobby/LobbyPlayerController.AddPlayerInfo` _aslobby_player_controller_2 (`self.ConnectedPlayers`))
      (`/Game/Blueprints/Lobby/LobbyPlayerController.UpdateAvailablePawns` _aslobby_player_controller_2 (`self.AvailablePawns`))
      (`self.AddToKickedList`))
    (for _array_element_3 (`self.ConnectedPlayers`) :!label _label
      (if (== (`.MyPlayerPawn_11_DA685ABF4EC53D5ACBE02B9A33955A4E` (break `/Game/Blueprints/AllLevels/StratagemaPlayerInfo` _array_element_3)) "/Game/Blueprints/Pawns/StratagemaPawn.StratagemaPawn_C")
        (set `self.ReadyToStart?` false)
        (`self.CannotStart`)
        (else
          (set `self.ReadyToStart?` true))))))

(event `YouHaveBeenKicked`
  (params (PlayerID :type Integer))
  ;[1 1 1] Kick Selected Player
  (`/Game/Blueprints/Lobby/LobbyPlayerController.Kicked` (cast `/Game/Blueprints/Lobby/LobbyPlayerController` (`KismetArrayLibrary.Array_Get` (`self.AllPlayerController`) PlayerID) :!pure true)))

(event `CannotStart`
  ;[1 1 1] Updates Connected Players
  (goto _label :!via `Break`))

(event `ServerUpdateGameSettings`
  (params (MapImage :type "Texture2D Object Reference") (MapName :type Text) (MapTime :type Text) (MapID :type Integer))
  ;[1 1 1] ServerChanged Update Clients
  (set `self.GameModeImage` MapImage)
  (set `self.GameModeMapName` MapName)
  (set `self.GameModeMapTime` MapTime)
  (set `self.GameModeMapID` MapID)
  (for _array_element (`self.AllPlayerController`)
    (bind _aslobby_player_controller (cast `/Game/Blueprints/Lobby/LobbyPlayerController` _array_element))
    (`/Game/Blueprints/Lobby/LobbyPlayerController.UpdateLobbySettings` _aslobby_player_controller (`self.GameModeImage`) (`self.GameModeMapName`) (`self.GameModeMapTime`))))

(event `LaunchGame`
  ;[1 1 1] Launch Game
  (`KismetSystemLibrary.ExecuteConsoleCommand` "servertravel /Game/Maps/StratagemaGame" (`GameplayStatics.GetPlayerController` 0)))

(fn `UserConstructionScript`)