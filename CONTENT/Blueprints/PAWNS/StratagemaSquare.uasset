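; StratagemaSquare turns a square of four nodes into a player's cube when the matching nodes beside it are also owned.
; DiscoverAndDrawCube finds the square's axis-aligned plane and box-traces from each corner to both sides, ignoring other StratagemaSquares.
; When all four hits on a side are owned nodes, FindCubeMinPoint anchors the center and SpawnCube spawns that PlayerID's cube class, unless colliding.
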(event `SpawnCube`
  (params (CubePosition :type "Vector Structure"))
  ;[0.7054 1 0.779] Spawn cube on server
  (switch `int` (`self.PlayerID`)
    (:`0`
      (set `self.PlayerCubeClass` "/Game/Blueprints/Pawns/CubeActor1.CubeActor1_C"))
    (:`1`
      (set `self.PlayerCubeClass` "/Game/Blueprints/Pawns/CubeActor2.CubeActor2_C"))
    (:`2`
      (set `self.PlayerCubeClass` "/Game/Blueprints/Pawns/CubeActor3.CubeActor3_C")))
  (`|SpawnActorFromClass` (`self.PlayerCubeClass`) (`KismetMathLibrary.MakeTransform` CubePosition (struct) (10.0 10.0 10.0)) "DontSpawnIfColliding" "OverrideRootScale"))

(event `DiscoverAndDrawCube`
  (params (Current :type "Vector Structure") (Adjacent1 :type "Vector Structure") (Adjacent2 :type "Vector Structure") (Opposite :type "Vector Structure") (OwnedNodes :type "Array of Actor Object Reference") (Player :type Integer))
  (bind _x (.x Current))
  (bind _y (.y Current))
  (bind _z (.z Current))
  (bind _x_2 (.x Adjacent1))
  (bind _y_2 (.y Adjacent1))
  (bind _z_2 (.z Adjacent1))
  (bind _x_3 (.x Adjacent2))
  (bind _y_3 (.y Adjacent2))
  (bind _z_3 (.z Adjacent2))
  (bind _x_4 (.x Opposite))
  (bind _y_4 (.y Opposite))
  (bind _z_4 (.z Opposite))
  (bind _returnvalue (- (`self.Opposite`) (0.0 0.0 400.0)))
  (bind _returnvalue_2 (- (`self.Current`) (0.0 0.0 400.0)))
  (bind _returnvalue_3 (- (`self.Adjcent 1`) (0.0 0.0 400.0)))
  (bind _returnvalue_4 (- (`self.Adjcent 2`) (0.0 0.0 400.0)))
  (bind _returnvalue_5 (- (`self.Current`) (400.0 0.0 0.0)))
  (bind _returnvalue_6 (- (`self.Adjcent 1`) (400.0 0.0 0.0)))
  (bind _returnvalue_7 (- (`self.Adjcent 2`) (400.0 0.0 0.0)))
  (bind _returnvalue_8 (- (`self.Opposite`) (400.0 0.0 0.0)))
  (bind _returnvalue_9 (- (`self.Current`) (0.0 400.0 0.0)))
  (bind _returnvalue_10 (- (`self.Adjcent 1`) (0.0 400.0 0.0)))
  (bind _returnvalue_11 (- (`self.Adjcent 2`) (0.0 400.0 0.0)))
  (bind _returnvalue_12 (- (`self.Opposite`) (0.0 400.0 0.0)))
  (bind _returnvalue_13 (+ (`self.Current`) (0.0 0.0 400.0)))
  (bind _returnvalue_14 (+ (`self.Adjcent 1`) (0.0 0.0 400.0)))
  (bind _returnvalue_15 (+ (`self.Adjcent 2`) (0.0 0.0 400.0)))
  (bind _returnvalue_16 (+ (`self.Opposite`) (0.0 0.0 400.0)))
  (bind _returnvalue_17 (+ (`self.Current`) (400.0 0.0 0.0)))
  (bind _returnvalue_18 (+ (`self.Adjcent 1`) (400.0 0.0 0.0)))
  (bind _returnvalue_19 (+ (`self.Adjcent 2`) (400.0 0.0 0.0)))
  (bind _returnvalue_20 (+ (`self.Opposite`) (400.0 0.0 0.0)))
  (bind _returnvalue_21 (+ (`self.Current`) (0.0 400.0 0.0)))
  (bind _returnvalue_22 (+ (`self.Adjcent 1`) (0.0 400.0 0.0)))
  (bind _returnvalue_23 (+ (`self.Adjcent 2`) (0.0 400.0 0.0)))
  (bind _returnvalue_24 (+ (`self.Opposite`) (0.0 400.0 0.0)))
  (bind _returnvalue_25 (and (== _z _z_2) (== _z_2 _z_3) (== _z_3 _z_4) (== _z_4 _z)))
  (bind _returnvalue_26 (and (== _x _x_2) (== _x_2 _x_3) (== _x_3 _x_4) (== _x_4 _x)))
  (bind _returnvalue_27 (and (== _y _y_2) (== _y_2 _y_3) (== _y_3 _y_4) (== _y _y_4)))
  (set `self.PlayerID` Player)
  (set `self.Current` Current)
  (set `self.Adjcent 1` Adjacent1)
  (set `self.Adjcent 2` Adjacent2)
  (set `self.Opposite` Opposite)
  (bind _outactors (`GameplayStatics.GetAllActorsOfClass` "StratagemaSquare_C"))
  (set `self.Ignore` _outactors)
  (set `self.ArrayOfOwnedNode` OwnedNodes)
  (`|ExecutionSequence`
    (:`then_0`
      ;[1 1 1] Cube X+
      (if _returnvalue_26
        (bind _outhit (`KismetSystemLibrary.BoxTraceSingle` _returnvalue_17 (+ _returnvalue_17 (100.0 0.0 0.0)) (50.0 50.0 50.0) (struct) "TraceTypeQuery1" false (`self.Ignore`)))
        (bind _outhit_2 (`KismetSystemLibrary.BoxTraceSingle` _returnvalue_18 (+ _returnvalue_18 (100.0 0.0 0.0)) (50.0 50.0 50.0) (struct) "TraceTypeQuery1" false (`self.Ignore`)))
        (bind _outhit_3 (`KismetSystemLibrary.BoxTraceSingle` _returnvalue_19 (+ _returnvalue_19 (100.0 0.0 0.0)) (50.0 50.0 50.0) (struct) "TraceTypeQuery1" false (`self.Ignore`)))
        (bind _outhit_4 (`KismetSystemLibrary.BoxTraceSingle` _returnvalue_20 (+ _returnvalue_20 (100.0 0.0 0.0)) (50.0 50.0 50.0) (struct) "TraceTypeQuery1" false (`self.Ignore`)))
        (if (and (`KismetArrayLibrary.Array_Contains` (`self.ArrayOfOwnedNode`) (`.HitActor` (`GameplayStatics.BreakHitResult` _outhit))) (`KismetArrayLibrary.Array_Contains` (`self.ArrayOfOwnedNode`) (`.HitActor` (`GameplayStatics.BreakHitResult` _outhit_2))) (`KismetArrayLibrary.Array_Contains` (`self.ArrayOfOwnedNode`) (`.HitActor` (`GameplayStatics.BreakHitResult` _outhit_3))) (`KismetArrayLibrary.Array_Contains` (`self.ArrayOfOwnedNode`) (`.HitActor` (`GameplayStatics.BreakHitResult` _outhit_4))))
          (bind _smallestposition (`self.FindCubeMinPoint` (`self.Current`) (`self.Adjcent 1`) (`self.Adjcent 2`) (`self.Opposite`)))
          (`self.SpawnCube` (+ _smallestposition (250.0 250.0 250.0))))))
    (:`then_1`
      (if _returnvalue_26
        ;[1 1 1] Cube x-
        (bind _outhit_5 (`KismetSystemLibrary.BoxTraceSingle` _returnvalue_5 (- _returnvalue_5 (100.0 0.0 0.0)) (50.0 50.0 50.0) (struct) "TraceTypeQuery1" false (`self.Ignore`)))
        (bind _outhit_6 (`KismetSystemLibrary.BoxTraceSingle` _returnvalue_6 (- _returnvalue_6 (100.0 0.0 0.0)) (50.0 50.0 50.0) (struct) "TraceTypeQuery1" false (`self.Ignore`)))
        (bind _outhit_7 (`KismetSystemLibrary.BoxTraceSingle` _returnvalue_7 (- _returnvalue_7 (100.0 0.0 0.0)) (50.0 50.0 50.0) (struct) "TraceTypeQuery1" false (`self.Ignore`)))
        (bind _outhit_8 (`KismetSystemLibrary.BoxTraceSingle` _returnvalue_8 (- _returnvalue_8 (100.0 0.0 0.0)) (50.0 50.0 50.0) (struct) "TraceTypeQuery1" false (`self.Ignore`)))
        (if (and (`KismetArrayLibrary.Array_Contains` (`self.ArrayOfOwnedNode`) (`.HitActor` (`GameplayStatics.BreakHitResult` _outhit_5))) (`KismetArrayLibrary.Array_Contains` (`self.ArrayOfOwnedNode`) (`.HitActor` (`GameplayStatics.BreakHitResult` _outhit_6))) (`KismetArrayLibrary.Array_Contains` (`self.ArrayOfOwnedNode`) (`.HitActor` (`GameplayStatics.BreakHitResult` _outhit_7))) (`KismetArrayLibrary.Array_Contains` (`self.ArrayOfOwnedNode`) (`.HitActor` (`GameplayStatics.BreakHitResult` _outhit_8))))
          (bind _smallestposition_2 (`self.FindCubeMinPoint` (`self.Current`) (`self.Adjcent 1`) (`self.Adjcent 2`) (`self.Opposite`)))
          (`self.SpawnCube` (- (+ _smallestposition_2 (0.0 250.0 250.0)) (250.0 0.0 0.0))))))
    (:`then_2`
      ;[1 1 1] Cube Y+
      (if _returnvalue_27
        (bind _outhit_9 (`KismetSystemLibrary.BoxTraceSingle` _returnvalue_21 (+ _returnvalue_21 (0.0 100.0 0.0)) (50.0 50.0 50.0) (struct) "TraceTypeQuery1" false (`self.Ignore`)))
        (bind _outhit_10 (`KismetSystemLibrary.BoxTraceSingle` _returnvalue_22 (+ _returnvalue_22 (0.0 100.0 0.0)) (50.0 50.0 50.0) (struct) "TraceTypeQuery1" false (`self.Ignore`)))
        (bind _outhit_11 (`KismetSystemLibrary.BoxTraceSingle` _returnvalue_23 (+ _returnvalue_23 (0.0 100.0 0.0)) (50.0 50.0 50.0) (struct) "TraceTypeQuery1" false (`self.Ignore`)))
        (bind _outhit_12 (`KismetSystemLibrary.BoxTraceSingle` _returnvalue_24 (+ _returnvalue_24 (0.0 100.0 0.0)) (50.0 50.0 50.0) (struct) "TraceTypeQuery1" false (`self.Ignore`)))
        (if (and (`KismetArrayLibrary.Array_Contains` (`self.ArrayOfOwnedNode`) (`.HitActor` (`GameplayStatics.BreakHitResult` _outhit_9))) (`KismetArrayLibrary.Array_Contains` (`self.ArrayOfOwnedNode`) (`.HitActor` (`GameplayStatics.BreakHitResult` _outhit_10))) (`KismetArrayLibrary.Array_Contains` (`self.ArrayOfOwnedNode`) (`.HitActor` (`GameplayStatics.BreakHitResult` _outhit_11))) (`KismetArrayLibrary.Array_Contains` (`self.ArrayOfOwnedNode`) (`.HitActor` (`GameplayStatics.BreakHitResult` _outhit_12))))
          (bind _smallestposition_3 (`self.FindCubeMinPoint` (`self.Current`) (`self.Adjcent 1`) (`self.Adjcent 2`) (`self.Opposite`)))
          (`self.SpawnCube` (+ _smallestposition_3 (250.0 250.0 250.0))))))
    (:`then_3`
      (if _returnvalue_27
        ;[1 1 1] Cube y-
        (bind _outhit_13 (`KismetSystemLibrary.BoxTraceSingle` _returnvalue_9 (- _returnvalue_9 (0.0 100.0 0.0)) (50.0 50.0 50.0) (struct) "TraceTypeQuery1" false (`self.Ignore`)))
        (bind _outhit_14 (`KismetSystemLibrary.BoxTraceSingle` _returnvalue_10 (- _returnvalue_10 (0.0 100.0 0.0)) (50.0 50.0 50.0) (struct) "TraceTypeQuery1" false (`self.Ignore`)))
        (bind _outhit_15 (`KismetSystemLibrary.BoxTraceSingle` _returnvalue_11 (- _returnvalue_11 (0.0 100.0 0.0)) (50.0 50.0 50.0) (struct) "TraceTypeQuery1" false (`self.Ignore`)))
        (bind _outhit_16 (`KismetSystemLibrary.BoxTraceSingle` _returnvalue_12 (- _returnvalue_12 (0.0 100.0 0.0)) (50.0 50.0 50.0) (struct) "TraceTypeQuery1" false (`self.Ignore`)))
        (if (and (`KismetArrayLibrary.Array_Contains` (`self.ArrayOfOwnedNode`) (`.HitActor` (`GameplayStatics.BreakHitResult` _outhit_13))) (`KismetArrayLibrary.Array_Contains` (`self.ArrayOfOwnedNode`) (`.HitActor` (`GameplayStatics.BreakHitResult` _outhit_14))) (`KismetArrayLibrary.Array_Contains` (`self.ArrayOfOwnedNode`) (`.HitActor` (`GameplayStatics.BreakHitResult` _outhit_15))) (`KismetArrayLibrary.Array_Contains` (`self.ArrayOfOwnedNode`) (`.HitActor` (`GameplayStatics.BreakHitResult` _outhit_16))))
          (bind _smallestposition_4 (`self.FindCubeMinPoint` (`self.Current`) (`self.Adjcent 1`) (`self.Adjcent 2`) (`self.Opposite`)))
          (`self.SpawnCube` (- (+ _smallestposition_4 (250.0 0.0 250.0)) (0.0 250.0 0.0))))))
    (:`then_4`
      ;[1 1 1] Cube Z+
      (if _returnvalue_25
        (bind _outhit_17 (`KismetSystemLibrary.BoxTraceSingle` _returnvalue_13 (+ _returnvalue_13 (0.0 0.0 100.0)) (50.0 50.0 50.0) (struct) "TraceTypeQuery1" false (`self.Ignore`)))
        (bind _outhit_18 (`KismetSystemLibrary.BoxTraceSingle` _returnvalue_14 (+ _returnvalue_14 (0.0 0.0 100.0)) (50.0 50.0 50.0) (struct) "TraceTypeQuery1" false (`self.Ignore`)))
        (bind _outhit_19 (`KismetSystemLibrary.BoxTraceSingle` _returnvalue_15 (+ _returnvalue_15 (0.0 0.0 100.0)) (50.0 50.0 50.0) (struct) "TraceTypeQuery1" false (`self.Ignore`)))
        (bind _outhit_20 (`KismetSystemLibrary.BoxTraceSingle` _returnvalue_16 (+ _returnvalue_16 (0.0 0.0 100.0)) (50.0 50.0 50.0) (struct) "TraceTypeQuery1" false (`self.Ignore`)))
        (if (and (`KismetArrayLibrary.Array_Contains` (`self.ArrayOfOwnedNode`) (`.HitActor` (`GameplayStatics.BreakHitResult` _outhit_17))) (`KismetArrayLibrary.Array_Contains` (`self.ArrayOfOwnedNode`) (`.HitActor` (`GameplayStatics.BreakHitResult` _outhit_18))) (`KismetArrayLibrary.Array_Contains` (`self.ArrayOfOwnedNode`) (`.HitActor` (`GameplayStatics.BreakHitResult` _outhit_19))) (`KismetArrayLibrary.Array_Contains` (`self.ArrayOfOwnedNode`) (`.HitActor` (`GameplayStatics.BreakHitResult` _outhit_20))))
          (bind _smallestposition_5 (`self.FindCubeMinPoint` (`self.Current`) (`self.Adjcent 1`) (`self.Adjcent 2`) (`self.Opposite`)))
          (`self.SpawnCube` (+ _smallestposition_5 (250.0 250.0 250.0))))))
    (:`then_5`
      (if _returnvalue_25
        ;[1 1 1] Cube Z -
        (bind _outhit_21 (`KismetSystemLibrary.BoxTraceSingle` _returnvalue_2 (- _returnvalue_2 (0.0 0.0 100.0)) (50.0 50.0 50.0) (struct) "TraceTypeQuery1" false (`self.Ignore`)))
        (bind _outhit_22 (`KismetSystemLibrary.BoxTraceSingle` _returnvalue_3 (- _returnvalue_3 (0.0 0.0 100.0)) (50.0 50.0 50.0) (struct) "TraceTypeQuery1" false (`self.Ignore`)))
        (bind _outhit_23 (`KismetSystemLibrary.BoxTraceSingle` _returnvalue_4 (- _returnvalue_4 (0.0 0.0 100.0)) (50.0 50.0 50.0) (struct) "TraceTypeQuery1" false (`self.Ignore`)))
        (bind _outhit_24 (`KismetSystemLibrary.BoxTraceSingle` _returnvalue (- _returnvalue (0.0 0.0 100.0)) (50.0 50.0 50.0) (struct) "TraceTypeQuery1" false (`self.Ignore`)))
        (if (and (`KismetArrayLibrary.Array_Contains` (`self.ArrayOfOwnedNode`) (`.HitActor` (`GameplayStatics.BreakHitResult` _outhit_21))) (`KismetArrayLibrary.Array_Contains` (`self.ArrayOfOwnedNode`) (`.HitActor` (`GameplayStatics.BreakHitResult` _outhit_22))) (`KismetArrayLibrary.Array_Contains` (`self.ArrayOfOwnedNode`) (`.HitActor` (`GameplayStatics.BreakHitResult` _outhit_23))) (`KismetArrayLibrary.Array_Contains` (`self.ArrayOfOwnedNode`) (`.HitActor` (`GameplayStatics.BreakHitResult` _outhit_24))))
          (bind _smallestposition_6 (`self.FindCubeMinPoint` (`self.Current`) (`self.Adjcent 1`) (`self.Adjcent 2`) (`self.Opposite`)))
          (`self.SpawnCube` (- (+ _smallestposition_6 (250.0 250.0 0.0)) (0.0 0.0 250.0))))))))

(event `self.ReceiveBeginPlay`)

(fn `FindCubeMinPoint`
  (params (Current :type "Vector Structure") (Adjcent1 :type "Vector Structure") (Adjcent2 :type "Vector Structure") (Opposite :type "Vector Structure"))
  (returns (SmallestPosition :type "Vector Structure"))
  (return (`KismetMathLibrary.MakeVector` (`.MinValue` (`KismetMathLibrary.MinOfFloatArray` (`|MakeArray` (.x Current) (.x Adjcent1) (.x Adjcent2) (.x Opposite)))) (`.MinValue` (`KismetMathLibrary.MinOfFloatArray` (`|MakeArray` (.y Current) (.y Adjcent1) (.y Adjcent2) (.y Opposite)))) (`.MinValue` (`KismetMathLibrary.MinOfFloatArray` (`|MakeArray` (.z Current) (.z Adjcent1) (.z Adjcent2) (.z Opposite)))))))

(fn `UserConstructionScript`)