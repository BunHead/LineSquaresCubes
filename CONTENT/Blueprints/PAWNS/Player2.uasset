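; Player 2 pawn for the Stratagema grid game, moving on X, Y and Z through six input actions.
; BeginPlay stores the second player's ID and finds the largest grid node coordinate to derive a camera offset.
; Space toggles between the pawn view and a spawned overview camera at that offset.
; Overlaps record owned grid nodes, increment Player 1's score (despite this being Player2) and call DefineAdjcentNodes.
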(event `InputAction|+XAxis`
  (params (Key :type "Key Structure" :default "AnyKey"))
  ;[1 1 1] Movement
  (:`Pressed`
    (`self.MoveX+`)))

(event `InputAction|-XAxis`
  (params (Key :type "Key Structure" :default "AnyKey"))
  ;[1 1 1] Movement
  (:`Pressed`
    (`self.MoveX-`)))

(event `InputAction|+YAxis`
  (params (Key :type "Key Structure" :default "AnyKey"))
  ;[1 1 1] Movement
  (:`Pressed`
    (`self.MoveY+`)))

(event `InputAction|-YAxis`
  (params (Key :type "Key Structure" :default "AnyKey"))
  ;[1 1 1] Movement
  (:`Pressed`
    (`self.MoveY-`)))

(event `InputAction|+ZAxis`
  (params (Key :type "Key Structure" :default "AnyKey"))
  ;[1 1 1] Movement
  (:`Pressed`
    (`self.MoveZ+`)))

(event `InputAction|-ZAxis`
  (params (Key :type "Key Structure" :default "AnyKey"))
  ;[1 1 1] Movement
  (:`Pressed`
    (`self.MoveZ-`)))

(event `Key|SpaceBar`
  (params (Key :type "Key Structure" :default "AnyKey"))
  (bind _returnvalue (`GameplayStatics.GetPlayerController` 0))
  ;[1 1 1] Space Bar Press
  (:`Pressed`
    (`/Engine/EditorBlueprintResources/StandardMacros.FlipFlop`
      (:`A`
        (bind _returnvalue_2 (`|SpawnActorFromClass` "/Script/Engine.CameraActor" (`KismetMathLibrary.MakeTransform` (`self.CameraOffset`) (struct :`Yaw` 45.0)) "AlwaysSpawn" "OverrideRootScale"))
        (`PlayerController.SetViewTargetWithBlend` _returnvalue _returnvalue_2 0.0 "VTBlend_Linear" 0.0 false))
      (:`B`
        (`PlayerController.SetViewTargetWithBlend` _returnvalue (`Controller.K2_GetPawn` _returnvalue) 0.0 "VTBlend_Linear" 0.0 false)
        (`/Engine/EditorBlueprintResources/StandardMacros.IsValid` _returnvalue_2
          (:`Is Valid`
            (`self.K2_DestroyActor` _returnvalue_2)))))))

(event `self.ReceiveBeginPlay`
  (bind _largestgridposition (`self.LargestGridPosition`))
  (bind _item (`KismetArrayLibrary.Array_Get` (`GameStateBase.PlayerArray` (`GameplayStatics.GetGameState`)) 1))
  ;[1 1 1] Begin Play
  (`parent.ReceiveBeginPlay`)
  (`/Engine/EditorBlueprintResources/StandardMacros.IsValid` _item
    (:`Is Valid`
      (set `self.Player2ID` (`PlayerState.PlayerId` _item))
      (bind _outactors (`GameplayStatics.GetAllActorsOfClass` "/Game/Blueprints/Pawns/StratagemaGridNode.StratagemaGridNode_C"))
      (for _array_element _outactors
        (bind (_returnvalue_x _returnvalue_y _returnvalue_z) (`KismetMathLibrary.BreakVector` (`SceneComponent.K2_GetComponentLocation` (`/Game/Blueprints/Pawns/StratagemaGridNode.NodeSphere` _array_element))))
        (`/Engine/EditorBlueprintResources/StandardMacros.CompareFloat` _returnvalue_x _largestgridposition
          (:`>`
            (bind _output_get (set `self.LargestGridPosition` _returnvalue_x)))
          (:`==`
            _)
          (:`<`
            _))
        (`/Engine/EditorBlueprintResources/StandardMacros.CompareFloat` _returnvalue_y _largestgridposition
          (:`>`
            (bind _output_get_2 (set `self.LargestGridPosition` _returnvalue_y)))
          (:`==`
            _)
          (:`<`
            _))
        (`/Engine/EditorBlueprintResources/StandardMacros.CompareFloat` _returnvalue_z _largestgridposition
          (:`>`
            (bind _output_get_3 (set `self.LargestGridPosition` _returnvalue_z)))))
      (set `self.CameraOffset` (`KismetMathLibrary.MakeVector` (* (/ _output_get 1.5) -1.0) (* (/ _output_get_2 1.5) -1.0) (/ _output_get_3 2.0))))))

(event `self.ReceiveActorBeginOverlap`
  (params (OtherActor :type "Actor Object Reference"))
  (bind _arrayofownednode (`self.ArrayOfOwnedNode`))
  ;[1 1 1] Update Player 1 Score on Move
  (bind _output_get (set `self.CurrentPosition` OtherActor))
  (if (not (`KismetArrayLibrary.Array_Contains` (`self.ArrayOfOwnedNode`) OtherActor))
    (`KismetArrayLibrary.Array_Add` _arrayofownednode _output_get)
    (bind _filteredarray (`KismetArrayLibrary.FilterArray` _arrayofownednode "/Game/Blueprints/Pawns/StratagemaGridNode.StratagemaGridNode_C"))
    (set `self.ArrayOfOwnedNode` _filteredarray))
  (`parent.ReceiveActorBeginOverlap` null)
  (bind _asstratageme_game_mode (cast `/Game/Blueprints/GamePlay/StratagemeGameMode` (`GameplayStatics.GetGameMode`)))
  (`/Game/Blueprints/GamePlay/StratagemeGameMode.Update Player 1 Score` _asstratageme_game_mode (+ (`/Game/Blueprints/GamePlay/StratagemeGameMode.Player1Score` _asstratageme_game_mode) 1))
  (`self.DefineAdjcentNodes`))

(fn `UserConstructionScript`
  (`parent.UserConstructionScript`))