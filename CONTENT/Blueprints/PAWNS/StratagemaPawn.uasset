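; Player pawn for a multiplayer node-capture game, stepping a sphere through a 3D node grid.
; Move events line-trace for a free or first-player-owned node, then slide the sphere with a beam trail; successes shorten move time, blocks lengthen it.
; DefineAdjcentNodes traces six neighbours for owned nodes, finds square corners and spawns a per-player square actor that runs DiscoverAndDrawCube.
; Tick passes the sphere's location to UpdateServer, which moves the actor.
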(event `self.ReceiveTick`
  (params (DeltaSeconds :type "Float (single-precision)"))
  ;[1 1 1] Update Server of Player Movement
  (`self.Update Server` (`SceneComponent.K2_GetComponentLocation` (`self.PlayerSphere`))))

(event `Update Server`
  (params (`Player Location` :type "Vector Structure"))
  ;[1 1 1] Update Sever
  (`self.K2_SetActorLocation` `Player Location`))

(event `self.ReceiveActorBeginOverlap`
  (params (OtherActor :type "Actor Object Reference")))

(event `self.ReceiveBeginPlay`)

(event `SpawnSquare`
  (bind _arrayofownednode (`self.ArrayOfOwnedNode`))
  (bind _adjcent_2 (`self.Adjcent 2`))
  (bind _adjcent_1 (`self.Adjcent 1`))
  (bind _testsquareopposite (`self.TestSquareOpposite`))
  (bind _returnvalue (`self.K2_GetActorLocation` (`self.CurrentPosition`)))
  (bind _playerarray (`GameStateBase.PlayerArray` (`GameplayStatics.GetGameState`)))
  ;[1 1 1] Spawn Square/Cube
  (if (== (`PlayerState.PlayerId` (`KismetArrayLibrary.Array_Get` _playerarray)) (`self.Player1ID`))
    (bind _returnvalue_2 (`|SpawnActorFromClass` "/Game/Blueprints/Pawns/SquareActor1.SquareActor1_C" (`KismetMathLibrary.MakeTransform` (`self.K2_GetActorLocation` (`self.CurrentPosition`)) (`self.DrawRotation`) (1.0 1.0 1.0)) "AlwaysSpawn" "OverrideRootScale"))
    (`/Game/Blueprints/Pawns/StratagemaSquare.DiscoverAndDrawCube` _returnvalue_2 _returnvalue _adjcent_1 _adjcent_2 _testsquareopposite _arrayofownednode 0)
    (elif (== (`PlayerState.PlayerId` (`KismetArrayLibrary.Array_Get` _playerarray 1)) (`self.Player2ID`))
      (bind _returnvalue_3 (`|SpawnActorFromClass` "/Game/Blueprints/Pawns/SquareActor2.SquareActor2_C" (`KismetMathLibrary.MakeTransform` (`self.K2_GetActorLocation` (`self.CurrentPosition`)) (`self.DrawRotation`) (1.0 1.0 1.0)) "AlwaysSpawn" "OverrideRootScale"))
      (`/Game/Blueprints/Pawns/StratagemaSquare.DiscoverAndDrawCube` _returnvalue_3 _returnvalue _adjcent_1 _adjcent_2 _testsquareopposite _arrayofownednode 1)
      (elif (== (`PlayerState.PlayerId` (`KismetArrayLibrary.Array_Get` _playerarray 2)) (`self.Player3ID`))
        (bind _returnvalue_4 (`|SpawnActorFromClass` "/Game/Blueprints/Pawns/SquareActor3.SquareActor3_C" (`KismetMathLibrary.MakeTransform` (`self.K2_GetActorLocation` (`self.CurrentPosition`)) (`self.DrawRotation`) (1.0 1.0 1.0)) "AlwaysSpawn" "OverrideRootScale"))
        (`/Game/Blueprints/Pawns/StratagemaSquare.DiscoverAndDrawCube` _returnvalue_4 _returnvalue _adjcent_1 _adjcent_2 _testsquareopposite _arrayofownednode 2)))))

(event `Key|SpaceBar`
  (params (Key :type "Key Structure" :default "AnyKey")))

(event `DefineAdjcentNodes`
  (bind _returnvalue (`self.K2_GetActorLocation` (`self.CurrentPosition`)))
  ;[1 1 1] Detect Adjacent Nodes and Compare to Array of Nodes
  (for _index (range 6)
    (switch `int` _index
      (:`0`
        (bind _output_get (set `self.TraceStart` (+ _returnvalue (0.0 0.0 400.0))))
        (set `self.TraceEnd` (+ _output_get (0.0 0.0 100.0))))
      (:`1`
        (bind _output_get_2 (set `self.TraceStart` (- _returnvalue (0.0 0.0 400.0))))
        (set `self.TraceEnd` (- _output_get_2 (0.0 0.0 100.0))))
      (:`2`
        (bind _output_get_3 (set `self.TraceStart` (+ _returnvalue (0.0 400.0 0.0))))
        (set `self.TraceEnd` (+ _output_get_3 (0.0 100.0 0.0))))
      (:`3`
        (bind _output_get_4 (set `self.TraceStart` (- _returnvalue (0.0 400.0 0.0))))
        (set `self.TraceEnd` (- _output_get_4 (0.0 100.0 0.0))))
      (:`4`
        (bind _output_get_5 (set `self.TraceStart` (+ _returnvalue (400.0 0.0 0.0))))
        (set `self.TraceEnd` (+ _output_get_5 (100.0 0.0 0.0))))
      (:`5`
        (bind _output_get_6 (set `self.TraceStart` (- _returnvalue (400.0 0.0 0.0))))
        (set `self.TraceEnd` (- _output_get_6 (100.0 0.0 0.0)))))
    (bind (_node_found _hitnodelocation) (`self.DetectNodesInArray` (`self.TraceStart`) (`self.TraceEnd`)))
    (if _node_found
      (if (!= (`self.TestSquareAdjCorner1`) (-1.0 -1.0 -1.0) :`ErrorTolerance` 0.0)
        (bind _output_get_7 (set `self.TestSquareAdjCorner2` _hitnodelocation))
        (set `self.Adjcent 2` _output_get_7)
        (`self.DefineOppositeNodes`)
        (else
          (bind _output_get_8 (set `self.TestSquareAdjCorner1` _hitnodelocation))
          (set `self.Adjcent 1` _output_get_8)))))
  (set `self.TestSquareAdjCorner1` (-1.0 -1.0 -1.0))
  (set `self.TestSquareAdjCorner2` (0.0 0.0 0.0)))

(event `DefineOppositeNodes`
  (bind _testsquareophighest (`self.TestSquareOpHighest`))
  (bind _testsquareoplowest (`self.TestSquareOpLowest`))
  (bind (_testsquareadjcorner2_x _testsquareadjcorner2_y _testsquareadjcorner2_z) (`KismetMathLibrary.BreakVector` (`self.TestSquareAdjCorner2`)))
  (bind (_testsquareadjcorner1_x _testsquareadjcorner1_y _testsquareadjcorner1_z) (`KismetMathLibrary.BreakVector` (`self.TestSquareAdjCorner1`)))
  (bind (_testsquareadjcorner1_x_2 _testsquareadjcorner1_y_2 _testsquareadjcorner1_z_2) (`KismetMathLibrary.BreakVector` (`self.TestSquareAdjCorner1`)))
  (bind (_testsquareadjcorner2_x_2 _testsquareadjcorner2_y_2 _testsquareadjcorner2_z_2) (`KismetMathLibrary.BreakVector` (`self.TestSquareAdjCorner2`)))
  (bind (_testsquareadjcorner2_x_3 _testsquareadjcorner2_y_3 _testsquareadjcorner2_z_3) (`KismetMathLibrary.BreakVector` (`self.TestSquareAdjCorner2`)))
  (bind (_testsquareadjcorner1_x_3 _testsquareadjcorner1_y_3 _testsquareadjcorner1_z_3) (`KismetMathLibrary.BreakVector` (`self.TestSquareAdjCorner1`)))
  (bind (_testsquareadjcorner1_x_4 _testsquareadjcorner1_y_4 _testsquareadjcorner1_z_4) (`KismetMathLibrary.BreakVector` (`self.TestSquareAdjCorner1`)))
  (bind (_testsquareadjcorner2_x_4 _testsquareadjcorner2_y_4 _testsquareadjcorner2_z_4) (`KismetMathLibrary.BreakVector` (`self.TestSquareAdjCorner2`)))
  (bind (_testsquareophighest_x _testsquareophighest_y _testsquareophighest_z) (`KismetMathLibrary.BreakVector` (`self.TestSquareOpHighest`)))
  (bind (_testsquareoplowest_x _testsquareoplowest_y _testsquareoplowest_z) (`KismetMathLibrary.BreakVector` (`self.TestSquareOpLowest`)))
  (bind (_testsquareophighest_x_2 _testsquareophighest_y_2 _testsquareophighest_z_2) (`KismetMathLibrary.BreakVector` (`self.TestSquareOpHighest`)))
  (bind (_testsquareoplowest_x_2 _testsquareoplowest_y_2 _testsquareoplowest_z_2) (`KismetMathLibrary.BreakVector` (`self.TestSquareOpLowest`)))
  (bind _testsquareophighest_2 (`self.TestSquareOpHighest`))
  (bind _testsquareoplowest_2 (`self.TestSquareOpLowest`))
  (bind _testsquareophighest_3 (`self.TestSquareOpHighest`))
  (bind _testsquareoplowest_3 (`self.TestSquareOpLowest`))
  (bind (_testsquareophighest_x_3 _testsquareophighest_y_3) (`KismetMathLibrary.BreakVector` (`self.TestSquareOpHighest`)))
  (bind (_testsquareoplowest_x_3 _testsquareoplowest_y_3) (`KismetMathLibrary.BreakVector` (`self.TestSquareOpLowest`)))
  (bind _returnvalue (> _testsquareophighest_y_3 _testsquareoplowest_y_3))
  (bind _returnvalue_2 (> _testsquareophighest_z _testsquareoplowest_z))
  (bind _returnvalue_3 (> _testsquareophighest_z_2 _testsquareoplowest_z_2))
  ;[1 1 1] Compare Final Node and Draw Square if Part of Array
  ;;[1 0 0] Does it in sequence
  (`|ExecutionSequence`
    (:`then_0`
      (if (== _testsquareadjcorner1_x _testsquareadjcorner2_x)
        (set `self.TestSquareOpLowest` (`KismetMathLibrary.MakeVector` _testsquareadjcorner1_x_3 _testsquareadjcorner2_y_3 _testsquareadjcorner1_z_3))
        (set `self.TestSquareOpHighest` (`KismetMathLibrary.MakeVector` _testsquareadjcorner2_x_3 _testsquareadjcorner1_y_3 _testsquareadjcorner2_z_3))
        (bind (_node_found _hitnodelocation) (`self.DetectNodesInArray` _testsquareoplowest_3 _testsquareophighest_3))
        (if (== _testsquareophighest_3 (`self.K2_GetActorLocation` (`self.CurrentPosition`)) :`ErrorTolerance` 5.0)
          (set `self.TestSquareOpposite` _hitnodelocation)
          (else
            (set `self.TestSquareOpposite` _testsquareoplowest_3)))
        (if _node_found
          (if (> _testsquareophighest_y _testsquareoplowest_y)
            (if _returnvalue_2
              ;;[1 1 1] Z- Y-
              (set `self.DrawRotation` (struct :`Yaw` -90.0 :`Roll` -90.0))
              (else
                ;;[1 1 1] Z+ Y-
                (set `self.DrawRotation` (struct :`Pitch` 90.0))))
            (elif _returnvalue_2
              ;;[1 1 1] Z- Y+
              (set `self.DrawRotation` (struct :`Yaw` 90.0 :`Roll` -90.0))
              (else
                ;;[1 1 1] Z+ Y+
                (set `self.DrawRotation` (struct :`Pitch` 90.0 :`Roll` 180.0)))))
          (`self.SpawnSquare` :!label _label))))
    (:`then_1`
      (if (== _testsquareadjcorner1_y _testsquareadjcorner2_y)
        (set `self.TestSquareOpLowest` (`KismetMathLibrary.MakeVector` _testsquareadjcorner1_x_2 _testsquareadjcorner1_y_2 _testsquareadjcorner2_z_2))
        (set `self.TestSquareOpHighest` (`KismetMathLibrary.MakeVector` _testsquareadjcorner2_x_2 _testsquareadjcorner2_y_2 _testsquareadjcorner1_z_2))
        (bind _node_found_2 (`self.DetectNodesInArray` _testsquareoplowest _testsquareophighest))
        (if (== _testsquareophighest (`self.K2_GetActorLocation` (`self.CurrentPosition`)) :`ErrorTolerance` 5.0)
          (set `self.TestSquareOpposite` _testsquareoplowest)
          (else
            (set `self.TestSquareOpposite` _testsquareophighest)))
        (if _node_found_2
          (if (> _testsquareophighest_x_2 _testsquareoplowest_x_2)
            (if _returnvalue_3
              ;;[1 1 1] X+ Z+
              (set `self.DrawRotation` (struct :`Roll` 90.0))
              (goto _label)
              (else
                ;;[1 1 1] X+ Z-
                (set `self.DrawRotation` (struct :`Pitch` -90.0 :`Yaw` 90.0))
                (goto _label)))
            (elif _returnvalue_3
              ;;[1 1 1] X- Z+
              (set `self.DrawRotation` (struct :`Yaw` 180.0 :`Roll` 90.0))
              (goto _label)
              (else
                ;;[1 1 1] X- Z-
                (set `self.DrawRotation` (struct :`Pitch` -90.0 :`Yaw` -90.0))
                (goto _label)))))))
    (:`then_2`
      (if (== _testsquareadjcorner2_z _testsquareadjcorner1_z)
        (set `self.TestSquareOpLowest` (`KismetMathLibrary.MakeVector` _testsquareadjcorner2_x_4 _testsquareadjcorner1_y_4 _testsquareadjcorner1_z_4))
        (set `self.TestSquareOpHighest` (`KismetMathLibrary.MakeVector` _testsquareadjcorner1_x_4 _testsquareadjcorner2_y_4 _testsquareadjcorner2_z_4))
        (bind (_node_found_3 _hitnodelocation_2) (`self.DetectNodesInArray` _testsquareoplowest_2 _testsquareophighest_2))
        (if (== _testsquareophighest_2 (`self.K2_GetActorLocation` (`self.CurrentPosition`)) :`ErrorTolerance` 5.0)
          (set `self.TestSquareOpposite` _testsquareoplowest_2)
          (else
            (set `self.TestSquareOpposite` _hitnodelocation_2)))
        (if _node_found_3
          (if (> _testsquareophighest_x_3 _testsquareoplowest_x_3)
            (if _returnvalue
              (set `self.DrawRotation` (struct :`Yaw` -90.0))
              (goto _label)
              (else
                (set `self.DrawRotation` (struct :`Yaw` 180.0))
                (goto _label)))
            (elif _returnvalue
              (set `self.DrawRotation` (struct))
              (goto _label)
              (else
                (set `self.DrawRotation` (struct :`Yaw` 90.0))
                (goto _label)))))))))

(event `MoveX+`
  (bind _returnvalue (`SceneComponent.K2_GetComponentLocation` (`self.PlayerSphere`)))
  (bind _returnvalue_2 (+ _returnvalue (0.0 500.0 0.0)))
  ;[1 0.5 0.5] X Axis
  (bind (_outhit _returnvalue_3) (`KismetSystemLibrary.LineTraceSingle` :`Start` (+ _returnvalue (0.0 400.0 0.0)) :`End` _returnvalue_2 :`TraceChannel` "TraceTypeQuery1" :`DrawTime` 0.1))
  (if _returnvalue_3
    (bind _returnvalue_4 (`KismetSystemLibrary.GetDisplayName` (`self.GetOwner` (`.HitActor` (`GameplayStatics.BreakHitResult` _outhit)))))
    (if (`KismetStringLibrary.EqualEqual_StrStr` _returnvalue_4)
      (`KismetSystemLibrary.MoveComponentTo` (`self.PlayerSphere`) _returnvalue_2 (struct) false false (`self.Speed`) :!label _label_2)
      (set `self.PathSource` (- _returnvalue (0.0 500.0 0.0)))
      (set `self.PathTarget` (- _returnvalue_2 (0.0 500.0 0.0)))
      (`self.SpawnEmitter` (`self.PathSource`) (`self.PathTarget`) (`self.PlayerEmiiter`) :!label _label_3)
      (set `self.Speed` (- (`self.Speed`) 0.05))
      (elif (`KismetStringLibrary.EqualEqual_StrStr` _returnvalue_4 (`KismetSystemLibrary.GetDisplayName` (`KismetArrayLibrary.Array_Get` (`GameState.PlayerArray` (`GameplayStatics.GetGameState`)))))
        (goto _label_2)
        (else
          (`KismetSystemLibrary.PrintString` "Node Captured" :!label _label_4)
          (`KismetSystemLibrary.PrintString` (`KismetSystemLibrary.GetDisplayName` (`self.GetOwner` (`.HitActor` (`GameplayStatics.BreakHitResult` (stale `MoveX-` _outhit)))))))))
    (else
      (`KismetSystemLibrary.PrintString` "Blocked Y" :!label _label_5)
      ;[0.5 1 0.5] Y Axis
      (`PlayerController.ClientStartCameraShake` :`self` (`GameplayStatics.GetPlayerController` 0) :`Shake` "/Game/Blueprints/Pawns/PlayerBlockedShake.PlayerBlockedShake_C" :`Scale` 1.0 :!label _label_6)
      (set `self.Speed` (+ (`self.Speed`) 0.2)))))

(event `MoveX-`
  (bind _returnvalue (`SceneComponent.K2_GetComponentLocation` (`self.PlayerSphere`)))
  (bind _returnvalue_2 (+ _returnvalue (0.0 -500.0 0.0)))
  ;[1 0.5 0.5] X Axis
  (bind (_outhit _returnvalue_3) (`KismetSystemLibrary.LineTraceSingle` :`Start` (+ _returnvalue (0.0 -400.0 0.0)) :`End` _returnvalue_2 :`TraceChannel` "TraceTypeQuery1" :`DrawTime` 0.1))
  (if _returnvalue_3
    (bind _returnvalue_4 (`KismetSystemLibrary.GetDisplayName` (`self.GetOwner` (`.HitActor` (`GameplayStatics.BreakHitResult` _outhit)))))
    (if (`KismetStringLibrary.EqualEqual_StrStr` _returnvalue_4)
      _
      (elif (`KismetStringLibrary.EqualEqual_StrStr` _returnvalue_4 (`KismetSystemLibrary.GetDisplayName` (`KismetArrayLibrary.Array_Get` (`GameState.PlayerArray` (`GameplayStatics.GetGameState`)))))
        _
        (else
          (goto _label_4))))
    (`KismetSystemLibrary.MoveComponentTo` (`self.PlayerSphere`) _returnvalue_2 (struct) false false (`self.Speed`))
    (set `self.PathSource` (+ _returnvalue (0.0 500.0 0.0)))
    (set `self.PathTarget` (+ _returnvalue_2 (0.0 500.0 0.0)))
    (goto _label_3)
    (else
      (goto _label_5))))

(event `MoveY+`
  (bind _returnvalue (`SceneComponent.K2_GetComponentLocation` (`self.PlayerSphere`)))
  (bind _returnvalue_2 (+ _returnvalue (500.0 0.0 0.0)))
  ;[0.5 1 0.5] Y Axis
  (bind (_outhit _returnvalue_3) (`KismetSystemLibrary.LineTraceSingle` :`Start` (+ _returnvalue (400.0 0.0 0.0)) :`End` _returnvalue_2 :`TraceChannel` "TraceTypeQuery1" :`DrawTime` 0.1))
  (if _returnvalue_3
    (bind _returnvalue_4 (`KismetSystemLibrary.GetDisplayName` (`self.GetOwner` (`.HitActor` (`GameplayStatics.BreakHitResult` _outhit)))))
    (if (`KismetStringLibrary.EqualEqual_StrStr` _returnvalue_4)
      (`KismetSystemLibrary.MoveComponentTo` (`self.PlayerSphere`) _returnvalue_2 (struct) false false (`self.Speed`) :!label _label_7)
      (set `self.PathSource` (- _returnvalue (500.0 0.0 0.0)))
      (set `self.PathTarget` (- _returnvalue_2 (500.0 0.0 0.0)))
      (goto _label_3)
      (elif (`KismetStringLibrary.EqualEqual_StrStr` _returnvalue_4 (`KismetSystemLibrary.GetDisplayName` (`KismetArrayLibrary.Array_Get` (`GameState.PlayerArray` (`GameplayStatics.GetGameState`)))))
        (goto _label_7)
        (else
          (`KismetSystemLibrary.PrintString` "Node Captured" :!label _label_8)
          (`KismetSystemLibrary.PrintString` (`KismetSystemLibrary.GetDisplayName` (`self.GetOwner` (`.HitActor` (`GameplayStatics.BreakHitResult` (stale `MoveY-` _outhit)))))))))
    (else
      (`KismetSystemLibrary.PrintString` "Blocked X" :!label _label_9)
      (goto _label_6))))

(event `MoveY-`
  (bind _returnvalue (`SceneComponent.K2_GetComponentLocation` (`self.PlayerSphere`)))
  (bind _returnvalue_2 (+ _returnvalue (-500.0 0.0 0.0)))
  ;[0.5 1 0.5] Y Axis
  (bind (_outhit _returnvalue_3) (`KismetSystemLibrary.LineTraceSingle` :`Start` (+ _returnvalue (-400.0 0.0 0.0)) :`End` _returnvalue_2 :`TraceChannel` "TraceTypeQuery1" :`DrawTime` 0.1))
  (if _returnvalue_3
    (bind _returnvalue_4 (`KismetSystemLibrary.GetDisplayName` (`self.GetOwner` (`.HitActor` (`GameplayStatics.BreakHitResult` _outhit)))))
    (if (`KismetStringLibrary.EqualEqual_StrStr` _returnvalue_4)
      _
      (elif (`KismetStringLibrary.EqualEqual_StrStr` _returnvalue_4 (`KismetSystemLibrary.GetDisplayName` (`KismetArrayLibrary.Array_Get` (`GameState.PlayerArray` (`GameplayStatics.GetGameState`)))))
        _
        (else
          (goto _label_8))))
    (`KismetSystemLibrary.MoveComponentTo` (`self.PlayerSphere`) _returnvalue_2 (struct) false false (`self.Speed`))
    (set `self.PathSource` (+ _returnvalue (500.0 0.0 0.0)))
    (set `self.PathTarget` (+ _returnvalue_2 (500.0 0.0 0.0)))
    (goto _label_3)
    (else
      (goto _label_9))))

(event `MoveZ+`
  (bind _returnvalue (`SceneComponent.K2_GetComponentLocation` (`self.PlayerSphere`)))
  (bind _returnvalue_2 (+ _returnvalue (0.0 0.0 500.0)))
  ;[0.65 0.737 5] Z Axis
  (bind (_outhit _returnvalue_3) (`KismetSystemLibrary.LineTraceSingle` :`Start` (+ _returnvalue (0.0 0.0 400.0)) :`End` _returnvalue_2 :`TraceChannel` "TraceTypeQuery1" :`DrawTime` 0.1))
  (if _returnvalue_3
    (bind _returnvalue_4 (`KismetSystemLibrary.GetDisplayName` (`self.GetOwner` (`.HitActor` (`GameplayStatics.BreakHitResult` _outhit)))))
    (if (`KismetStringLibrary.EqualEqual_StrStr` _returnvalue_4)
      (`KismetSystemLibrary.MoveComponentTo` (`self.PlayerSphere`) _returnvalue_2 (struct) false false (`self.Speed`) :!label _label_10)
      (set `self.PathSource` (- _returnvalue (0.0 0.0 500.0)))
      (set `self.PathTarget` (- _returnvalue_2 (0.0 0.0 500.0)))
      (goto _label_3)
      (elif (`KismetStringLibrary.EqualEqual_StrStr` _returnvalue_4 (`KismetSystemLibrary.GetDisplayName` (`KismetArrayLibrary.Array_Get` (`GameState.PlayerArray` (`GameplayStatics.GetGameState`)))))
        (goto _label_10)
        (else
          (`KismetSystemLibrary.PrintString` "Node Captured by" :!label _label_11)
          (`KismetSystemLibrary.PrintString` (`KismetSystemLibrary.GetDisplayName` (`self.GetOwner` (`.HitActor` (`GameplayStatics.BreakHitResult` (stale `MoveZ-` _outhit)))))))))
    (else
      (`KismetSystemLibrary.PrintString` "Blocked Z" :!label _label_12)
      (goto _label_6))))

(event `MoveZ-`
  (bind _returnvalue (`SceneComponent.K2_GetComponentLocation` (`self.PlayerSphere`)))
  (bind _returnvalue_2 (+ _returnvalue (0.0 0.0 -500.0)))
  ;[0.65 0.737 5] Z Axis
  (bind (_outhit _returnvalue_3) (`KismetSystemLibrary.LineTraceSingle` :`Start` (+ _returnvalue (0.0 0.0 -400.0)) :`End` _returnvalue_2 :`TraceChannel` "TraceTypeQuery1" :`DrawTime` 0.1))
  (if _returnvalue_3
    (bind _returnvalue_4 (`KismetSystemLibrary.GetDisplayName` (`self.GetOwner` (`.HitActor` (`GameplayStatics.BreakHitResult` _outhit)))))
    (if (`KismetStringLibrary.EqualEqual_StrStr` _returnvalue_4)
      _
      (elif (`KismetStringLibrary.EqualEqual_StrStr` _returnvalue_4 (`KismetSystemLibrary.GetDisplayName` (`KismetArrayLibrary.Array_Get` (`GameState.PlayerArray` (`GameplayStatics.GetGameState`)))))
        _
        (else
          (goto _label_11))))
    (`KismetSystemLibrary.MoveComponentTo` (`self.PlayerSphere`) _returnvalue_2 (struct) false false (`self.Speed`))
    (set `self.PathSource` (+ _returnvalue (0.0 0.0 500.0)))
    (set `self.PathTarget` (+ _returnvalue_2 (0.0 0.0 500.0)))
    (goto _label_3)
    (else
      (goto _label_12))))

(fn `DetectNodesInArray`
  (params (Start :type "Vector Structure") (End :type "Vector Structure"))
  (returns (`Node Found` :type Boolean) (HitNodeLocation :type "Vector Structure"))
  (bind _outhit (`KismetSystemLibrary.LineTraceSingle` :`Start` Start :`End` End :`TraceChannel` "TraceTypeQuery1" :`DrawTime` 2.0))
  (bind (_bblockinghit _binitialoverlap _time _location _impactpoint _normal _impactnormal _physmat _hitactor) (`GameplayStatics.BreakHitResult` _outhit))
  (if (`KismetArrayLibrary.Array_Contains` (`self.ArrayOfOwnedNode`) _hitactor)
    (return true (`self.K2_GetActorLocation` _hitactor))
    (else
      (return false (0.0 0.0 0.0)))))

(fn `SpawnEmitter`
  (params (Current :type "Vector Structure") (Destination :type "Vector Structure") (Emitter :type "ParticleSystem Object Reference"))
  (bind _returnvalue (`GameplayStatics.SpawnEmitterAtLocation` Emitter Current (struct) false))
  (`ParticleSystemComponent.SetBeamEndPoint` _returnvalue 0 Destination))

(fn `UserConstructionScript`)