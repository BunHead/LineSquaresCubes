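; StratagemaGridNode is a grid node Blueprint that labels a node and reports its position in grid units.
; SetNodeName splits the target's display name on underscores and stores the first segment plus the last segment, trimmed at any dot, as CurrentNode.
; GetNodeMatrix divides the target's world location by 500 and returns it as formatted text with CurrentNode.
; The event graph and construction script contain no logic.
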(fn `GetNodeMatrix`
  (params (Target :type "PrimitiveComponent Object Reference"))
  (returns (`Current Node` :type Text))
  (bind (_returnvalue_x _returnvalue_y _returnvalue_z) (`KismetMathLibrary.BreakVector` (`SceneComponent.K2_GetComponentLocation` Target)))
  (bind _output_get (set `self.X` _returnvalue_x))
  (bind _output_get_2 (set `self.Y` _returnvalue_y))
  (bind _output_get_3 (set `self.Z` _returnvalue_z))
  (return (`|FormatText` "@ Position {X} , {Y} , {Z} = {Ref}" (`KismetTextLibrary.Conv_DoubleToText` (/ _returnvalue_x 500.0) "HalfToEven") (`KismetTextLibrary.Conv_DoubleToText` (/ _returnvalue_y 500.0) "HalfToEven") (`KismetTextLibrary.Conv_DoubleToText` (/ _returnvalue_z 500.0) "HalfToEven") (`self.CurrentNode`))))

(fn `SetNodeName`
  (params (Target :type "PrimitiveComponent Object Reference"))
  (bind _returnvalue (`KismetStringLibrary.ParseIntoArray` (`KismetSystemLibrary.GetDisplayName` Target) "_" false))
  (for _array_element _returnvalue
    (set `self.CurrentNode` (`|FormatText` "{Node}{Number}" (`KismetTextLibrary.Conv_StringToText` (`KismetArrayLibrary.Array_Get` _returnvalue)) (`KismetTextLibrary.Conv_StringToText` (`KismetArrayLibrary.Array_Get` (`KismetStringLibrary.ParseIntoArray` _array_element "." false)))))))

(fn `UserConstructionScript`)